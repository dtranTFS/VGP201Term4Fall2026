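; Health component for the FPS game that stores a clamped health value between configurable minimum and maximum bounds.
; Heal, Damage, HealFull, Kill and Setup all route through SetHealth, which clamps the value and fires a health-updated notification.
; Heal and Damage only accept positive amounts and print a message otherwise, while helper functions report death and normalized health percentage.
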(fn `ClampHealth`
  (params (Health :type "Float (double-precision)"))
  (returns (Value :type "Float (double-precision)"))
  (return (`KismetMathLibrary.FClamp` Health (`self.MinHealth`) (`self.MaxHealth`))))

(fn `Damage`
  (params (Amount :type "Float (double-precision)"))
  (if (> Amount 0.0)
    (`self.SetHealth` (- (`self.GetHealth`) Amount))
    (else
      (`KismetSystemLibrary.PrintString` "Hey why are you stupid. Its a positive idiot"))))

(fn `GetHealth`
  (returns (Value :type "Float (double-precision)"))
  (return (`self.Health`)))

(fn `GetPercentHealth`
  (returns (Value :type "Float (double-precision)"))
  (return (`KismetMathLibrary.FClamp` (/ (- (`self.GetHealth`) (`self.MinHealth`)) (- (`self.MaxHealth`) (`self.MinHealth`))))))

(fn `Heal`
  (params (Amount :type "Float (double-precision)"))
  (if (> Amount 0.0)
    (`self.SetHealth` (+ (`self.GetHealth`) Amount))
    (else
      (`KismetSystemLibrary.PrintString` "Hey why are you stupid. Its a positive idiot"))))

(fn `HealFull`
  (`self.Heal` (`self.MaxHealth`)))

(fn `IsDead`
  (returns (Value :type Boolean))
  (return (<= (`self.GetHealth`) (`self.MinHealth`))))

(fn `Kill`
  (`self.Damage` (`self.MaxHealth`)))

(fn `SetHealth`
  (params (NewHealth :type "Float (double-precision)"))
  (returns (Value :type "Float (double-precision)"))
  (bind _output_get (set `self.Health` (`self.ClampHealth` NewHealth)))
  (`self.OnHealthUpdated`)
  (return _output_get))

(fn `Setup`
  (params (Health :type "Float (double-precision)") (MinHealth :type "Float (double-precision)") (MaxHealth :type "Float (double-precision)"))
  (set `self.MinHealth` MinHealth)
  (set `self.MaxHealth` MaxHealth)
  (`self.SetHealth` Health))