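; BP_EnemyCharacter is an FPS enemy character that takes damage and is removed when its health runs out.
; On BeginPlay it initializes ACHealthComponent with a small health pool and binds a handler to its health-updated event.
; AnyDamage forwards incoming damage to the component, and the handler destroys the actor once the component reports it is dead.
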(event `self.ReceiveBeginPlay`
  (bind _ac_healthcomponent (`self.AC_HealthComponent`))
  (`/Game/FPS/Components/AC_HealthComponent.Setup` _ac_healthcomponent 10.0 0.0 10.0)
  (add `/Game/FPS/Components/AC_HealthComponent.OnHealthUpdated` _ac_healthcomponent (delegate `OnDamage`)))

(event `OnDamage`
  (if (`/Game/FPS/Components/AC_HealthComponent.IsDead` (`self.AC_HealthComponent`))
    (`self.K2_DestroyActor`)))

(event `self.ReceiveAnyDamage`
  (params (Damage :type "Float (single-precision)") (DamageType :type "DamageType Object Reference") (InstigatedBy :type "Controller Object Reference") (DamageCauser :type "Actor Object Reference"))
  (`/Game/FPS/Components/AC_HealthComponent.Damage` (`self.AC_HealthComponent`) Damage))

(fn `UserConstructionScript`)