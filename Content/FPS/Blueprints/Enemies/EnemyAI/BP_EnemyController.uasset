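; AI controller for the FPS enemy that runs the BT_EnemyAI behavior tree on BeginPlay.
; PawnSensing sightings of BP_Player write the player and a CanSeePlayer flag to the Blackboard.
; A retriggerable delay of twice the sensing interval clears both keys once sightings stop, acting as a lose-sight timeout.
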(event `self.ReceiveBeginPlay`
  (`self.RunBehaviorTree` "/Game/FPS/Blueprints/Enemies/EnemyAI/BT_EnemyAI.BT_EnemyAI"))

(event `self.PawnSensing.OnSeePawn`
  (params (Pawn :type "Pawn Object Reference"))
  (bind _asbp_player (cast `/Game/FPS/Blueprints/BP_Player` Pawn))
  (`self.SetBlackboardCanSeePlayer` _asbp_player true)
  (`KismetSystemLibrary.RetriggerableDelay` (* (`PawnSensingComponent.SensingInterval` (`self.PawnSensing`)) 2.0))
  (`self.SetBlackboardCanSeePlayer` null))

(fn `SetBlackboardCanSeePlayer`
  (params (ObjectValue :type "Object Object Reference") (BoolValue :type Boolean))
  (`BlackboardComponent.SetValueAsBool` (`self.Blackboard`) (`self.CanSeePlayerKeyName`) BoolValue)
  (`BlackboardComponent.SetValueAsObject` (`self.Blackboard`) (`self.PlayerKeyName`) ObjectValue))

(fn `UserConstructionScript`)