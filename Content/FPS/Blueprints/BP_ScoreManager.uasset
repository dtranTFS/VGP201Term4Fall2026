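; BP_ScoreManager tracks the player's score in the FPS game and pushes it to the game menu UI.
; AddToScore adds an amount to Score, refreshes the display and returns the new total.
; UpdateScoreUI reaches the WBP_GameMenu widget through the GameMenuRef on BP_GameManager, the game mode.
; BeginPlay waits one frame before showing the initial score.
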(event `self.ReceiveBeginPlay`
  (`KismetSystemLibrary.DelayUntilNextFrame`)
  (`self.UpdateScoreUI`))

(fn `AddToScore`
  (params (Amount :type Integer))
  (returns (Score :type Integer))
  (bind _output_get (set `self.Score` (+ (`self.Score`) Amount)))
  (`self.UpdateScoreUI`)
  (return _output_get))

(fn `UpdateScoreUI`
  (bind _asbp_game_manager (cast `/Game/FPS/Blueprints/BP_GameManager` (`GameplayStatics.GetGameMode`)))
  (bind _aswbp_game_menu (cast `/Game/FPS/Blueprints/GUI/Game/WBP_GameMenu` (`/Game/FPS/Blueprints/BP_GameManager.GameMenuRef` _asbp_game_manager)))
  (`/Game/FPS/Blueprints/GUI/Game/WBP_GameMenu.UpdateScore` _aswbp_game_menu (`self.Score`)))

(fn `UserConstructionScript`)