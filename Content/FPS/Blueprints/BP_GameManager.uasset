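; BP_GameManager runs the match countdown and tracks game over in the FPS game.
; On BeginPlay it spawns the game menu widget, sets game-only input and binds to the player's death event, which sets IsGameOver.
; Tick drives a Delay-based macro that lowers the zero-clamped timer once a second and refreshes the UI, or prints a message once the game is over.
; Reaching zero does not end the game, and a score-increment snippet is unconnected.
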(event `self.ReceiveBeginPlay`
  (`self.SpawnGameMenu` "/Game/FPS/Blueprints/GUI/Game/WBP_GameMenu.WBP_GameMenu_C")
  (`self.SetInputMode` false)
  (`self.UpdateTimerUI`)
  (bind _asbp_player (cast `/Game/FPS/Blueprints/BP_Player` (`GameplayStatics.GetPlayerCharacter` 0)))
  (add `/Game/FPS/Blueprints/BP_Player.OnPlayerDied` _asbp_player (delegate `OnPlayerDied`)))

(event `OnPlayerDied`
  (set `self.IsGameOver` true))

(event `self.ReceiveTick`
  (params (DeltaSeconds :type "Float (single-precision)"))
  (if (`self.IsGameOver`)
    (`KismetSystemLibrary.PrintString` "Game is over")
    (else
      (`self.DecreaseTimer`)
      (`self.UpdateTimerUI`))))

(fn `SetInputMode`
  (params (`Show Mouse Cursor` :type Boolean) (InWidgetToFocus :type "Widget Object Reference"))
  (bind _returnvalue (`GameplayStatics.GetPlayerController` 0))
  (if `Show Mouse Cursor`
    (`WidgetBlueprintLibrary.SetInputMode_UIOnlyEx` (`GameplayStatics.GetPlayerController` 0) InWidgetToFocus)
    (else
      (`WidgetBlueprintLibrary.SetInputMode_GameOnly` _returnvalue)))
  (set `PlayerController.bShowMouseCursor` `Show Mouse Cursor` _returnvalue))

(fn `SpawnGameMenu`
  (params (Class :type "UserWidget Class Reference"))
  (bind _returnvalue (`|CreateWidget` Class))
  (bind _output_get (set `self.GameMenuRef` _returnvalue))
  (`UserWidget.AddToViewport` _output_get 0))

(fn `UpdateTimerUI`
  (bind _aswbp_game_menu (cast `/Game/FPS/Blueprints/GUI/Game/WBP_GameMenu` (`self.GameMenuRef`)))
  (`/Game/FPS/Blueprints/GUI/Game/WBP_GameMenu.UpdateTimer` _aswbp_game_menu (`self.GameTimer`)))

(fn `UserConstructionScript`)