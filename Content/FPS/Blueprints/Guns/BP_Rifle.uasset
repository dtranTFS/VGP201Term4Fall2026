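; BP_Rifle is a hitscan rifle Blueprint that extends its parent's OnBlueprintShoot event to damage whatever it hits.
; CalculateShoot projects a ray from the given camera's location along its forward vector for ShootDistance.
; OnBlueprintShoot calls the parent, line-traces that ray on the Visibility channel, then applies Damage to the hit actor.
; Debug output is left on, drawing each trace and printing the hit actor's name.
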(fn `CalculateShoot`
  (params (Camera :type "SceneComponent Object Reference"))
  (returns (Start :type "Vector Structure") (End :type "Vector Structure"))
  (bind _returnvalue (`SceneComponent.K2_GetComponentLocation` Camera))
  (return _returnvalue (+ _returnvalue (* (`SceneComponent.GetForwardVector` Camera) (`self.ShootDistance`)))))

(fn `OnBlueprintShoot`
  (params (Camera :type "CameraComponent Object Reference"))
  (bind (_start _end) (`self.CalculateShoot` Camera))
  (`parent.OnBlueprintShoot` Camera)
  (bind (_outhit _returnvalue) (`KismetSystemLibrary.LineTraceSingle` :`Start` _start :`End` _end :`TraceChannel` "TraceTypeQuery1" :`DrawDebugType` "ForDuration"))
  (if _returnvalue
    (bind (_bblockinghit _binitialoverlap _time _distance _location _impactpoint _normal _impactnormal _physmat _hitactor) (`GameplayStatics.BreakHitResult` _outhit))
    (`KismetSystemLibrary.PrintString` (`KismetSystemLibrary.GetDisplayName` _hitactor))
    (`GameplayStatics.ApplyDamage` _hitactor (`self.Damage`))))

(fn `UserConstructionScript`
  (`parent.UserConstructionScript`))