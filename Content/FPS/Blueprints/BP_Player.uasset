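; BP_Player is the playable FPS character, handling Enhanced Input movement, look, jump and shooting.
; On BeginPlay it adds its input mapping, attaches a spawned BP_Rifle at GunSpawnPoint and sets up ACHealthComponent.
; Fire sends the camera to the gun through interface messages, immediately on press, then repeatedly while triggered via a Delay set by the gun's fire rate.
; Health updates reach the WBP_GameMenu health bar through BP_GameManager, the game mode.
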(event `self.ReceiveBeginPlay`
  (`self.SetupEnhancedInput`)
  (`self.SpawnGun` "/Game/FPS/Blueprints/Guns/BP_Rifle.BP_Rifle_C" (`SceneComponent.GetRelativeTransform` (`self.GunSpawnPoint`)))
  (add `/Game/FPS/Components/AC_HealthComponent.OnHealthUpdated` (`self.AC_HealthComponent`) (delegate `OnHealthUpdated`))
  (`/Game/FPS/Components/AC_HealthComponent.Setup` (`self.AC_HealthComponent`) 100.0 0.0 100.0))

(event `OnHealthUpdated`
  (`self.UpdateHealthBarUI`))

(event `EnhancedInput|/Game/FPS/Input/IA_Move`
  (params (ActionValue :type "Vector2D Structure") (ElapsedSeconds :type "Float (double-precision)") (TriggeredSeconds :type "Float (double-precision)") (InputAction :type "InputAction Object Reference" :default "/Game/FPS/Input/IA_Move.IA_Move"))
  (bind (_x _y) (`KismetMathLibrary.BreakVector2D` ActionValue))
  ; Movement
  (:`Triggered`
    (`self.AddMovementInput` (`self.GetActorForwardVector`) _y)
    (`self.AddMovementInput` (`self.GetActorRightVector`) _x)))

(event `EnhancedInput|/Game/FPS/Input/IA_Jump`
  (params (ActionValue :type Boolean) (ElapsedSeconds :type "Float (double-precision)") (TriggeredSeconds :type "Float (double-precision)") (InputAction :type "InputAction Object Reference" :default "/Game/FPS/Input/IA_Jump.IA_Jump"))
  ; Jumping
  (:`Started`
    (`self.Jump`))
  (:`Completed`
    (`self.StopJumping`)))

(event `EnhancedInput|/Game/FPS/Input/IA_Look`
  (params (ActionValue :type "Vector2D Structure") (ElapsedSeconds :type "Float (double-precision)") (TriggeredSeconds :type "Float (double-precision)") (InputAction :type "InputAction Object Reference" :default "/Game/FPS/Input/IA_Look.IA_Look"))
  (bind (_x _y) (`KismetMathLibrary.BreakVector2D` ActionValue))
  ; Look
  (:`Triggered`
    (`self.AddControllerYawInput` _x)
    (`self.AddControllerPitchInput` _y)))

(event `EnhancedInput|/Game/FPS/Input/IA_Fire`
  (params (ActionValue :type "Float (double-precision)") (ElapsedSeconds :type "Float (double-precision)") (TriggeredSeconds :type "Float (double-precision)") (InputAction :type "InputAction Object Reference" :default "/Game/FPS/Input/IA_Fire.IA_Fire"))
  ; Shooting
  (:`Triggered`
    (bind _value (message `/Game/FPS/Blueprints/Guns/BPI_IGun.GetFireRate` (`self.GunRef`)))
    (`KismetSystemLibrary.Delay` _value)
    (message `/Game/FPS/Blueprints/Guns/BPI_IGun.OnInterfaceShoot` (`self.GunRef`) (`self.Camera`) :!label _label))
  (:`Started`
    (goto _label)))

(fn `SetupEnhancedInput`
  (bind _asplayer_controller (cast `PlayerController` (`self.GetController`)))
  (`EnhancedInputSubsystemInterface.AddMappingContext` (pcsubsystem `EnhancedInputLocalPlayerSubsystem` _asplayer_controller) "/Game/FPS/Input/IMC_Player.IMC_Player" 0 (struct)))

(fn `SpawnGun`
  (params (Spawn :type "Actor Class Reference") (SpawnTransform :type "Transform Structure"))
  (bind _returnvalue (`|SpawnActorFromClass` Spawn SpawnTransform "Undefined" "MultiplyWithRoot" null null))
  (bind _output_get (set `self.GunRef` _returnvalue))
  (`self.K2_AttachToComponent` _output_get (`self.GunSpawnPoint`) "None" "SnapToTarget" "SnapToTarget" "SnapToTarget" true))

(fn `UpdateHealthBarUI`
  (bind _asbp_game_manager (cast `/Game/FPS/Blueprints/BP_GameManager` (`GameplayStatics.GetGameMode`)))
  (bind _aswbp_game_menu (cast `/Game/FPS/Blueprints/GUI/Game/WBP_GameMenu` (`/Game/FPS/Blueprints/BP_GameManager.GameMenuRef` _asbp_game_manager)))
  (`/Game/FPS/Blueprints/GUI/Game/WBP_GameMenu.UpdateHealthBar` _aswbp_game_menu (`/Game/FPS/Components/AC_HealthComponent.GetPercentHealth` (`self.AC_HealthComponent`))))

(fn `UserConstructionScript`)